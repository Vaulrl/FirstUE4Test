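; Game instance that acts as the central UI manager for a survival game, opening and closing the runtime HUD, message box, pickable, inventory, cabinet and failure panels.
; ShowPanel lazily creates each widget, caches it by reference and adds it to the viewport.
; Interactive panels increment an active UI count and enable Game-and-UI input with cursor.
; HidePanel decrements the count, restoring game-only input at zero.
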(event `ShowRuntimeUI`
  (`self.ShowPanel` (`self.RuntimeUI`) "/Game/UI/UI_RuntimeUI.UI_RuntimeUI_C")
  (`self.ShowPanel` (`self.MessageBox`) "/Game/UI/UI_MeesageBox.UI_MeesageBox_C"))

(event `PushMessage`
  (params (textContent :type Text))
  (`/Game/UI/UI_MeesageBox.PushMessage` (`self.MessageBox`) textContent))

(event `ShowPickablePanel`
  (`self.ShowPanel` (`self.PickablePanel`) "/Game/UI/UI_PickablePanel.UI_PickablePanel_C" true))

(event `HidePickablePanel`
  (`self.HidePanel` (`self.PickablePanel`)))

(event `ShowInventoryPannel`
  (`self.ShowPanel` (`self.InventoryPanel`) "/Game/UI/UI_Inventory.UI_Inventory_C" true))

(event `HideInventoryPanel`
  (`self.HidePanel` (`self.InventoryPanel`)))

(event `ShowCabinetPanel`
  (`self.ShowPanel` (`self.CabinetUI`) "/Game/UI/UI_Cabinet.UI_Cabinet_C" true))

(event `HideCabinetPanel`
  (`self.HidePanel` (`self.CabinetUI`)))

(event `ShowFailedPanel`
  (`self.ShowPanel` (`self.FailedPanel`) "/Game/UI/UI_Failed.UI_Failed_C" true))

(event `HideAllPanels`
  (`self.HidePanel` (`self.InventoryPanel`))
  (`self.HidePanel` (`self.PickablePanel`))
  (`self.HidePanel` (`self.CabinetUI`)))

(fn `HidePanel`
  (params (PanelVar :type "Widget Object Reference"))
  (bind _returnvalue (`GameplayStatics.GetPlayerController` 0))
  (`/Engine/EditorBlueprintResources/StandardMacros.IsValid` PanelVar
    (:`Is Valid`
      (if (`Widget.IsVisible` PanelVar)
        (`Widget.RemoveFromParent` PanelVar)
        (bind _result (`/Engine/EditorBlueprintResources/StandardMacros.DecrementInt` (`self.ActiveUICount`))
          (:`  `
            (if (== _result 0)
              (`WidgetBlueprintLibrary.SetInputMode_GameOnly` _returnvalue)
              (set `PlayerController.bShowMouseCursor` false _returnvalue))))))))

(fn `ShowPanel`
  (params (PanelVariable :type "UserWidget Object Reference (by ref)") (PanelTypeClass :type "UserWidget Class Reference") (bChangeUIMod :type Boolean))
  (bind _returnvalue (`GameplayStatics.GetPlayerController` 0))
  (`/Engine/EditorBlueprintResources/StandardMacros.IsValid` PanelVariable
    (:`Is Valid`
      (if (not (`Widget.IsInViewport` PanelVariable))
        (`UserWidget.AddToViewport` PanelVariable 0 :!label _label)
        (if bChangeUIMod
          (`/Engine/EditorBlueprintResources/StandardMacros.IncrementInt` (`self.ActiveUICount`)
            (:`  `
              (`WidgetBlueprintLibrary.SetInputMode_GameAndUIEx` _returnvalue PanelVariable)
              (set `PlayerController.bShowMouseCursor` true _returnvalue))))))
    (:`Is Not Valid`
      (bind _returnvalue_2 (`|CreateWidget` PanelTypeClass (`GameplayStatics.GetPlayerController` 0)))
      (`|VariableSetRef` PanelVariable _returnvalue_2)
      (goto _label))))